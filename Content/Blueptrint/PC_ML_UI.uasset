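; Player controller that opens the game's UI screens: album (Carte), aiming display (visée), menu and start screen.
; Each function creates its widget, stores it and adds it to the viewport; album, aiming and start reuse a valid instance.
; The menu is recreated on every call with UI-only input, showing the cursor only if a previous menu exists.
; The album always shows the cursor.
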(event EventBeginPlay)

(event EventTick
  (params (DeltaSeconds :type Float%20%28single-precision%29)))

(fn ConstructionScript)

(fn UIShowCarte
  (Variables|Default|SetbShowMouseCursor true)
  (Utilities|IsValid (Variables|Default|GetWB_album)
    (:Is%20Valid
      _)
    (:Is%20Not%20Valid
      (bind _returnvalue (UserInterface|CreateWidget "/Game/UI/WBP_Album.WBP_Album_C" self))
      (Variables|Default|SetWB_album _returnvalue)))
  (UserInterface|Viewport|AddtoViewport (Variables|Default|GetWB_album) 0))

(fn UIVisée
  (Utilities|IsValid (Variables|Default|GetWB_visée)
    (:Is%20Valid
      _)
    (:Is%20Not%20Valid
      (bind _returnvalue (UserInterface|CreateWidget "/Game/Blueptrint/WBP_visée.WBP_visée_C" self))
      (Variables|Default|SetWB_visée _returnvalue)))
  (UserInterface|Viewport|AddtoViewport (Variables|Default|GetWB_visée) 0))

(fn UIMenu
  (Utilities|IsValid (Variables|Default|GetWB_menu)
    (:Is%20Valid
      (Variables|/Script/Engine.PlayerController|SetbShowMouseCursor (Game|GetPlayerController 0) true))
    (:Is%20Not%20Valid
      _))
  (bind _returnvalue (UserInterface|CreateWidget "/Game/UI/WBP_Menu.WBP_Menu_C" self))
  (Input|SetInputModeUIOnly 0 _returnvalue "DoNotLock" false)
  (Variables|Default|SetWB_menu _returnvalue)
  (UserInterface|Viewport|AddtoViewport (Variables|Default|GetWB_menu) 0))

(fn UIStart
  (Utilities|IsValid (Variables|Default|GetWB_start)
    (:Is%20Valid
      _)
    (:Is%20Not%20Valid
      (bind _returnvalue (UserInterface|CreateWidget "/Game/UI/WBP_Start.WBP_Start_C" self))
      (Variables|Default|SetWB_start _returnvalue)))
  (UserInterface|Viewport|AddtoViewport (Variables|Default|GetWB_start) 0))