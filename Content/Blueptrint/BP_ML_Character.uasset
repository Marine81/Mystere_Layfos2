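; First-person player character that handles object interaction and physics grabbing, and calls the aiming UI on PC_ML at BeginPlay.
; Left click line-traces from the camera and casts the hit actor to pick up violin pieces, play a trigger object's widget or collect health.
; Holding right click grabs the component hit by a shorter trace with a PhysicsHandle, which Tick keeps in front of the camera until release.
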(event EventBeginPlay
  (bind _asbp_ml_character (Utilities|Casting|CastToBP_ML_Character (Game|GetPlayerCharacter 0)))
  (bind _aspc_ml (Utilities|Casting|CastToPC_ML (Pawn|GetController _asbp_ml_character)))
  (Default|UIVisée _aspc_ml))

(event EventTick
  (params (DeltaSeconds :type Float%20%28single-precision%29))
  (bind _firstpersoncamera (Variables|Default|GetFirstPersonCamera))
  (if (Variables|Default|Getisgrabbing?)
    (Physics|Components|PhysicsHandle|SetTargetLocation (Variables|Default|GetPhysicsHandle) (+ (Transformation|GetWorldLocation _firstpersoncamera) (* (Math|Vector|GetForwardVector (Transformation|GetWorldRotation _firstpersoncamera)) 2e+02)))))

(event Input|MouseEvents|RightMouseButton
  (params (Key :type Key%20Structure :default "None"))
  (bind _firstpersoncamera (Variables|Default|GetFirstPersonCamera))
  (bind _returnvalue (Transformation|GetWorldLocation _firstpersoncamera))
  (:Pressed
    (bind (_outhit _returnvalue_2) (Collision|LineTraceByChannel _returnvalue (+ _returnvalue (* (Math|Vector|GetForwardVector (Transformation|GetWorldRotation _firstpersoncamera)) 2e+02)) "TraceTypeQuery1" false 0 "None"))
    (if _returnvalue_2
      (Physics|Components|PhysicsHandle|GrabComponentatLocationwithRotation (Variables|Default|GetPhysicsHandle) (.HitComponent (Collision|BreakHitResult _outhit)) "None" (Transformation|GetWorldLocation (.HitComponent (Collision|BreakHitResult _outhit))) "0, 0, 0")
      (Variables|Default|Setisgrabbing? true)))
  (:Released
    (if (Variables|Default|Getisgrabbing?)
      (Physics|Components|PhysicsHandle|ReleaseComponent (Variables|Default|GetPhysicsHandle))
      (Variables|Default|Setisgrabbing? false))))

(event Input|MouseEvents|LeftMouseButton
  (params (Key :type Key%20Structure :default "None"))
  (bind _firstpersoncamera (Variables|Default|GetFirstPersonCamera))
  (bind _returnvalue (Transformation|GetWorldLocation _firstpersoncamera))
  (:Pressed
    (bind _outhit (Collision|LineTraceByChannel _returnvalue (+ _returnvalue (* (Math|Vector|GetForwardVector _firstpersoncamera) 5e+02)) "TraceTypeQuery1" false 0 "None"))
    (bind _asmorceau_violon (Utilities|Casting|CastToMorceau_violon (.HitActor (Collision|BreakHitResult _outhit)))
      (:then
        (Default|Ramasser _asmorceau_violon))
      (:CastFailed
        (bind _as_objetdeclencheur (Utilities|Casting|CastTo_Objetdeclencheur (.HitActor (Collision|BreakHitResult _outhit)))
          (:then
            (Default|LectureWidget _as_objetdeclencheur))
          (:CastFailed
            (bind _asrecuperation_vie (Utilities|Casting|CastToRecuperation_vie (.HitActor (Collision|BreakHitResult _outhit))))
            (Default|RecupVie _asrecuperation_vie)))))))

(fn ConstructionScript)